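; Test-pattern video Blueprint for the VP base system that plays a media source with keyboard transport controls.
; BeginPlay enables input for player controller 0, opens the SpiderMan source on MediaP and lowers or raises TAA current-frame weight by console command.
; Space toggles play and pause.
; Left and Right pause, seek by SkipTime seconds, then resume after a short delay, even if playback was paused.
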(event EventBeginPlay
  ;[1 1 1] 미디어 플레이어 시작 (init)
  (Input|EnableInput (Game|GetPlayerController 0))
  (Media|MediaPlayer|OpenSource (Variables|Default|GetMedia_P) "/Game/Media/SpiderMan.SpiderMan")
  (Development|ExecuteConsoleCommand "r.TemporalAACurrentFrameWeight 0.2" 0))

(event Input|KeyboardEvents|SpaceBar
  (params (Key :type Key%20Structure :default "None"))
  (bind _media_p (Variables|Default|GetMedia_P))
  ;[1 1 1] 미디어 플레이어 정지 및 시작
  (:Pressed
    (if (Audio|Components|Audio|IsPlaying (Variables|Default|GetMedia_P))
      (Sequencer|Player|Pause _media_p)
      (else
        (Media|MediaPlayer|Play _media_p :!class /Script/MediaAssets.MediaPlayer)))))

(event Input|KeyboardEvents|Left
  (params (Key :type Key%20Structure :default "None"))
  (bind _media_p (Variables|Default|GetMedia_P))
  (bind _returnvalue (Class|MediaPlayer|GetTime _media_p))
  (bind (_days _hours _minutes _seconds _milliseconds) (Math|Timespan|BreakTimespan _returnvalue))
  ;[1 1 1] 탐색 뒤로 이동
  (:Pressed
    (Sequencer|Player|Pause _media_p)
    (Media|MediaPlayer|Seek _media_p (Math|Timespan|MakeTimespan _days _hours _minutes (+ _seconds (* (Variables|Default|GetSkipTime) -1)) _milliseconds))
    (Utilities|FlowControl|Delay 0.2)
    (Media|MediaPlayer|Play (Variables|Default|GetMedia_P) :!class /Script/MediaAssets.MediaPlayer)))

(event Input|KeyboardEvents|Right
  (params (Key :type Key%20Structure :default "None"))
  (bind _media_p (Variables|Default|GetMedia_P))
  (bind _returnvalue (Class|MediaPlayer|GetTime _media_p))
  (bind (_days _hours _minutes _seconds _milliseconds) (Math|Timespan|BreakTimespan _returnvalue))
  ;[1 1 1] 탐색 앞으로 이동
  (:Pressed
    (Sequencer|Player|Pause _media_p)
    (Media|MediaPlayer|Seek _media_p (Math|Timespan|MakeTimespan _days _hours _minutes (+ _seconds (* (Variables|Default|GetSkipTime) 1)) _milliseconds))
    (Utilities|FlowControl|Delay 0.2)
    (Media|MediaPlayer|Play (Variables|Default|GetMedia_P) :!class /Script/MediaAssets.MediaPlayer)))

(fn ConstructionScript)