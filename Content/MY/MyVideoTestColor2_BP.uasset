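; MyVideoTestColor2_BP is a test Blueprint that plays a video through a media player.
; On BeginPlay it enables input for the first player controller, opens the SpiderMan media source and raises the temporal AA current-frame weight by console command.
; The space bar toggles the player between pause and play.
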(event EventBeginPlay
  ;[1 1 1] 미디어 플레이어 시작 (init)
  (Input|EnableInput (Game|GetPlayerController 0))
  (Media|MediaPlayer|OpenSource (Variables|Default|GetMedia_P) "/Game/Media/SpiderMan.SpiderMan")
  (Development|ExecuteConsoleCommand "r.TemporalAACurrentFrameWeight 0.2" 0))

(event Collision|EventActorBeginOverlap
  (params (OtherActor :type Actor%20Object%20Reference)))

(event EventTick
  (params (DeltaSeconds :type Float%20%28single-precision%29)))

(event Input|KeyboardEvents|SpaceBar
  (params (Key :type Key%20Structure :default "None"))
  (bind _media_p (Variables|Default|GetMedia_P))
  ;[1 1 1] 코멘트
  (:Pressed
    (if (Audio|Components|Audio|IsPlaying (Variables|Default|GetMedia_P))
      (Sequencer|Player|Pause _media_p)
      (else
        (Media|MediaPlayer|Play _media_p :!class /Script/MediaAssets.MediaPlayer)))))

(fn ConstructionScript)